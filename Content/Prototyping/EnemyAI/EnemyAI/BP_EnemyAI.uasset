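; Enemy AI character that patrols, chases the player on sight and sends them back to their checkpoint when caught.
; Tick picks chase, waypoint-loop patrol or random roaming via AIMoveTo, each at its own walk speed.
; PawnSensing sets visibility, which lapses through a retriggerable delay after last sighting.
; Attack montage notify sphere-traces from the hand to trigger checkpoint loading; AttackBox overlap also attacks and loads it immediately.
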(event OnSeePawn(PawnSensing)
  (params (Pawn :type Pawn%20Object%20Reference))
  (Utilities|FlowControl|Sequence
    (:then_0
      (Components|Activation|Activate (Variables|Default|GetAudio) false)
      (Utilities|Casting|CastToBP_ThirdPersonCharacter Pawn
        (:then
          (Variables|Default|SetBPlaverVisable true)
          (Utilities|FlowControl|DoOnce false :!label _label
            (:Completed
              (Development|PrintString ""))))
        (:CastFailed
          (Variables|Default|SetBPlaverVisable false))))
    (:then_1
      (Utilities|FlowControl|RetriggerableDelay 1.0)
      (Variables|Default|SetBPlaverVisable false)
      (Development|PrintString "")
      (goto _label Reset))))

(event OnComponentBeginOverlap(Attackbox)
  (params (OverlappedComponent :type Primitive%20Component%20Object%20Reference) (OtherActor :type Actor%20Object%20Reference) (OtherComp :type Primitive%20Component%20Object%20Reference) (OtherBodyIndex :type Integer) (bFromSweep :type Boolean) (SweepResult :type Hit%20Result%20Structure%20%28by%20ref%29))
  (bind _asbp_third_person_character (Utilities|Casting|CastToBP_ThirdPersonCharacter OtherActor))
  (CallFunction|Attack)
  (Default|LoadCheckpoint _asbp_third_person_character))

(event Custom|Chase%20Player
  (CallFunction|UpdateWalkSpeed 4.5e+02)
  (Variables|Default|SetBCanMove false)
  (AI|AIMoveTo self "0, 0, 0" (Game|GetPlayerCharacter 0) 5.0 false
    (:OnSuccess
      (Utilities|FlowControl|Delay 0.2)
      (CallFunction|Attack)
      (Variables|Default|SetBCanMove true))))

(event Custom|Attack
  (bind _mesh (Variables|Character|GetMesh))
  (bind _returnvalue (Transformation|GetSocketLocation _mesh "hand_r"))
  ;[0.15 0.1407 0.04319 0.5] Bonk
  (Utilities|FlowControl|DoOnce false ; Only Reset Attack on miss.
    (:Completed
      (bind _notifyname (Animation|Montage|PlayMontage (Variables|Character|GetMesh) "/Game/Prototyping/EnemyAI/AM_Attack_01.AM_Attack_01") ; Play the AM_Attack_01
        (:OnCompleted
          (Audio|Components|Audio|Play (Variables|Default|Getattacknoise) 0.0)
          (CallFunction|ResetAttack) ; Resets the Do Once node.
        )
        (:OnNotifyBegin
          (switch name _notifyname ; Pick the proper attack type(standard when there is more than one type of attack)
            (:AttackDamage
              (Development|PrintString "I'm attacking!")
              (bind (_outhits _returnvalue_2) (Collision|MultiSphereTraceForObjects _returnvalue (+ _returnvalue (* (Transformation|GetActorForwardVector) (Variables|Default|GetMeleeTraceDistance))) (Variables|Default|GetMeleeTraceRadius) (Utilities|Array|MakeArray "ObjectTypeQuery3") false 0 "None")) ; Trace forward from hand socket.
              (if _returnvalue_2 ; If a pawn is hit in that trace...
                (for _array_element _outhits ; ...loop through the results....
                  (bind _asbp_third_person_character (Utilities|Casting|CastToBP_ThirdPersonCharacter (.HitActor (Collision|BreakHitResult _array_element))))
                  (Default|LoadCheckpoint _asbp_third_person_character)
                  (Development|PrintString "Bonk"))))))))))

(event Custom|Move%20to%20next%20Patrol%20Point
  (CallFunction|UpdateWalkSpeed 2e+02)
  (Variables|Default|SetBCanMove false)
  (AI|AIMoveTo self "0, 0, 0" (Utilities|Array|Get(acopy) (Variables|Default|GetPatrolTargetPoints) (Variables|Default|GetPatrolTargetPointIndex)) 5.0 false
    (:OnSuccess
      (Utilities|FlowControl|Delay 3.0)
      (Variables|Default|SetBCanMove true)
      (CallFunction|SetNextPatrolPointIndex))))

(event Custom|ResetAttack
  (bind _mesh (Variables|Character|GetMesh))
  (bind _returnvalue (Transformation|GetSocketLocation _mesh "hand_r"))
  ;[0.15 0.1407 0.04319 0.5] Bonk
  (Utilities|FlowControl|DoOnce false) ; enters at Reset
)

(event Custom|Patrol%20Random
  (CallFunction|UpdateWalkSpeed 375.0)
  (Variables|Default|SetBCanMove false)
  (AI|AIMoveTo self (.RandomLocation (AI|Navigation|GetRandomReachablePointinRadius (Transformation|GetActorLocation) 2e+04 0 0)) 0 5.0 false
    (:OnSuccess
      (Utilities|FlowControl|Delay 3.0)
      (Variables|Default|SetBCanMove true))))

(event Custom|Set%20next%20Patrol%20Point%20Index
  (Variables|Default|SetPatrolTargetPointIndex (Math|Integer|%(Integer) (+ (Variables|Default|GetPatrolTargetPointIndex) 1) (Utilities|Array|Length (Variables|Default|GetPatrolTargetPoints)))))

(event EventBeginPlay)

(event Collision|EventActorBeginOverlap
  (params (OtherActor :type Actor%20Object%20Reference)))

(event EventTick
  (params (DeltaSeconds :type Float%20%28single-precision%29))
  (bind _bplavervisable (Variables|Default|GetBPlaverVisable))
  (if (Variables|Default|GetBCanMove)
    (if _bplavervisable
      (CallFunction|ChasePlayer)
      (elif (Variables|Default|GetBTargetPointMovement)
        (CallFunction|MovetoNextPatrolPoint)
        (else
          (CallFunction|PatrolRandom))))
    (elif _bplavervisable
      (CallFunction|ChasePlayer))))

(fn ConstructionScript)

(fn UpdateWalkSpeed
  (params (NewWalkSpeed :type Float%20%28double-precision%29))
  (Variables|/Script/Engine.CharacterMovementComponent|SetMaxWalkSpeed (Variables|Character|GetCharacterMovement) NewWalkSpeed))